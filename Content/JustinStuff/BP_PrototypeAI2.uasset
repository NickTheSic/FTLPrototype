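; BP_PrototypeAI2 is a prototype enemy bot that runs BT_PrototypeAI and fires at the player.
; BeginPlay sets the player as the blackboard target, optionally pre-triggering the bot, and AI perception updates CanSeePlayer.
; Each tick it calls Fire while alive, if blackboard flags show it triggered and seeing a target within MaxDistance.
; Tick also sets StopFiring once the test game mode reports the player dead.
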(event OnTargetPerceptionUpdated(AIPerception)
  (params (Actor :type Actor%20Object%20Reference) (Stimulus :type AI%20Stimulus%20Structure))
  (bind _self self)
  (bind _returnvalue (AI|GetBlackboard _self))
  (bind _asfirst_person_character (Utilities|Casting|CastToFirstPersonCharacter Actor))
  (Variables|Default|SetPlayer _asfirst_person_character)
  (Utilities|IsValid _returnvalue
    (:Is%20Valid
      (AI|Components|Blackboard|SetValueasBool _returnvalue (Utilities|Name|MakeLiteralName "CanSeePlayer") (.bSuccessfullySensed (Utilities|Struct|BreakAIStimulus Stimulus))))))

(event EventBeginPlay
  (bind _self self)
  (bind _returnvalue (AI|GetBlackboard _self))
  (AI|RunBehaviorTree (AI|GetAIController self) "/Game/JustinStuff/BT_PrototypeAI.BT_PrototypeAI")
  (bind _asfirst_person_character (Utilities|Casting|CastToFirstPersonCharacter (Game|Player|GetPlayerPawn 0)))
  (AI|Components|Blackboard|SetValueasObject (AI|GetBlackboard self) (Utilities|Name|MakeLiteralName "TargetActor") _asfirst_person_character)
  ;[1 1 1] Enable/Disable Trigger at start (Automatically chases player if on!)
  (if (Variables|Default|GetEnableTriggerAtStart)
    (AI|Components|Blackboard|SetValueasBool _returnvalue (Utilities|Name|MakeLiteralName "Trigger") true)
    (AI|Components|Blackboard|SetValueasBool _returnvalue (Utilities|Name|MakeLiteralName "CanSeePlayer") true)
    (Development|PrintString "Bot Spawned" true true "(R=0.000000,G=0.660000,B=1.000000,A=1.000000)" 5.0)))

(event EventTick
  (params (DeltaSeconds :type Float%20%28single-precision%29))
  ;[1 1 1] RESET
  (Utilities|FlowControl|Sequence
    (:then_0
      (CallFunction|IsAbletoFire))
    (:then_1
      (bind _asbp_test_game_mode (Utilities|Casting|CastToBP_TestGameMode (Game|GetGameMode)))
      (if (Variables|/Game/JustinStuff/BP_TestGameMode.BP_TestGameMode_C|GetPlayerDead _asbp_test_game_mode)
        (Utilities|FlowControl|DoOnce false
          (:Completed
            ;[1 1 1] Stops firing when player is dead
            (Variables|Default|SetStopFiring true)))))))

(fn ConstructionScript)

(fn IsAbletoFire
  (bind _self self)
  (bind _returnvalue (AI|GetBlackboard _self))
  (if (not (Variables|/Script/FTLPrototype.FTLPrototypeHealthComponent|GetbIsDead (Variables|Default|GetHealthComp)))
    (if (and (ScalableFloat|GetValueasBool _returnvalue (Utilities|Name|MakeLiteralName "Triggered")) (ScalableFloat|GetValueasBool _returnvalue (Utilities|Name|MakeLiteralName "CanSeePlayer")))
      (bind _asactor (Utilities|Casting|CastToActor (AI|Components|Blackboard|GetValueasObject _returnvalue (Utilities|Name|MakeLiteralName "TargetActor"))))
      (if (<= (Math|Vector|VectorLength (- (Transformation|GetActorLocation _asactor) (Transformation|GetActorLocation))) (Variables|Default|GetMaxDistance))
        (Class|FTLPrototypeAI|Fire)))))