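; Test game mode that continuously spawns AI enemies and restarts the level when the player dies.
; A looping timer runs an EQS query for a spawn location, then spawns BP_PrototypeAI2 there with a debug sphere.
; Tick treats a player pawn that fails the FTLPrototypeCharacter cast as death, printing a message once and reopening the hard-coded FirstPersonExampleMap after a delay.
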(event Custom|OnQueryFinishedEvent
  (params (QueryInstance :type Env%20Query%20Instance%20Blueprint%20Wrapper%20Object%20Reference) (QueryStatus :type EEnvQueryStatus%20Enum :default "Processing"))
  (switch Utilities|FlowControl|Switch|SwitchonEEnvQueryStatus QueryStatus
    (:Success
      (bind _resultlocations (AI|EQS|GetQueryResultsasLocations QueryInstance))
      (for _array_element _resultlocations
        (Rendering|Debug|DrawDebugSphere _array_element 1e+02 12 "(R=1.000000,G=1.000000,B=1.000000,A=1.000000)" 0.0)
        (Game|SpawnActorfromClass "/Game/JustinStuff/BP_PrototypeAI2.BP_PrototypeAI2_C" (Math|Transform|MakeTransform _array_element) "AdjustIfPossibleButAlwaysSpawn" (Components|GetOwner) 0)))))

(event Custom|SpawnAI
  (bind _returnvalue (AI|EQS|RunEQSQuery "/Game/JustinStuff/SpawningStuff/EQS_FindSpawnLocation.EQS_FindSpawnLocation" self "SingleResult"))
  (EventDispatchers|BindEventtoOnQueryFinishedEvent _returnvalue (delegate Custom|OnQueryFinishedEvent)))

(event EventBeginPlay
  (Utilities|Time|SetTimerbyEvent (delegate Custom|SpawnAI) 2.0 true))

(event EventTick
  (params (DeltaSeconds :type Float%20%28single-precision%29))
  (Utilities|Casting|CastToFTLPrototypeCharacter (Game|Player|GetPlayerPawn 0)
    (:CastFailed
      (Utilities|FlowControl|DoOnce false
        (:Completed
          (Development|PrintString "Dead")
          (Utilities|FlowControl|Delay 3.2)
          ;[1 1 1] IF the level doesnt restart, CHANGE THIS!
          (Game|OpenLevel(byName) "FirstPersonExampleMap"))))))

(fn ConstructionScript)