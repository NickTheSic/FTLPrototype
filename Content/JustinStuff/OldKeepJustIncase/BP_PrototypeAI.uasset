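; BP_PrototypeAI is a prototype AI that fires at the player.
; BeginPlay runs BT_PrototypeAI and stores the player pawn as the blackboard's TargetActor.
; AI perception updates write CanSeePlayer to the blackboard and print a debug message.
; Each Tick, IsAbleToFire calls Fire if the AI is alive, the blackboard flags Triggered and CanSeePlayer are set, and the target is within MaxDistance.
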(event OnTargetPerceptionUpdated(AIPerception)
  (params (Actor :type Actor%20Object%20Reference) (Stimulus :type AI%20Stimulus%20Structure))
  (AI|Components|Blackboard|SetValueasBool (AI|GetBlackboard self) (Utilities|Name|MakeLiteralName "CanSeePlayer") (.bSuccessfullySensed (Utilities|Struct|BreakAIStimulus Stimulus)))
  (Development|PrintString "Hello"))

(event EventBeginPlay
  (AI|RunBehaviorTree (AI|GetAIController self) "/Game/JustinStuff/BT_PrototypeAI.BT_PrototypeAI")
  (AI|Components|Blackboard|SetValueasObject (AI|GetBlackboard self) (Utilities|Name|MakeLiteralName "TargetActor") (Game|Player|GetPlayerPawn 0)))

(event EventTick
  (params (DeltaSeconds :type Float%20%28single-precision%29))
  (CallFunction|IsAbletoFire))

(fn ConstructionScript)

(fn IsAbletoFire
  (bind _self self)
  (bind _returnvalue (AI|GetBlackboard _self))
  (if (not (Variables|/Script/FTLPrototype.FTLPrototypeHealthComponent|GetbIsDead (Variables|Default|GetHealthComp)))
    (if (and (ScalableFloat|GetValueasBool _returnvalue (Utilities|Name|MakeLiteralName "Triggered")) (ScalableFloat|GetValueasBool _returnvalue (Utilities|Name|MakeLiteralName "CanSeePlayer")))
      (bind _asactor (Utilities|Casting|CastToActor (AI|Components|Blackboard|GetValueasObject _returnvalue (Utilities|Name|MakeLiteralName "TargetActor"))))
      (if (<= (Math|Vector|VectorLength (- (Transformation|GetActorLocation _asactor) (Transformation|GetActorLocation))) (Variables|Default|GetMaxDistance))
        (Class|FTLPrototypeAI|Fire)))))